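; TutorialArea is a trigger volume that supplies tutorial text to the player while occupied.
; When a component tagged Body enters AutomaticTrigger, it copies its TutorialText to the Player_Polished character and sets that character's TutorialActivated flag.
; When such a component leaves, it clears the flag.
; Both events act on player character 0 rather than on the overlapping actor.
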(event OnComponentBeginOverlap(AutomaticTrigger)
  (params (OverlappedComponent :type Primitive%20Component%20Object%20Reference) (OtherActor :type Actor%20Object%20Reference) (OtherComp :type Primitive%20Component%20Object%20Reference) (OtherBodyIndex :type Integer) (bFromSweep :type Boolean) (SweepResult :type Hit%20Result%20Structure%20%28by%20ref%29))
  (if (Components|ComponentHasTag OtherComp "Body")
    (bind _asplayer_polished (Utilities|Casting|CastToPlayer_Polished (Game|GetPlayerCharacter 0)))
    (Variables|/Game/Blueprints/Players/Player_Polished.Player_Polished_C|SetTutorialTexts _asplayer_polished (Variables|Default|GetTutorialText))
    (Variables|/Game/Blueprints/Players/Player_Polished.Player_Polished_C|SetTutorialActivated _asplayer_polished true)))

(event OnComponentEndOverlap(AutomaticTrigger)
  (params (OverlappedComponent :type Primitive%20Component%20Object%20Reference) (OtherActor :type Actor%20Object%20Reference) (OtherComp :type Primitive%20Component%20Object%20Reference) (OtherBodyIndex :type Integer))
  (if (Components|ComponentHasTag OtherComp "Body")
    (bind _asplayer_polished (Utilities|Casting|CastToPlayer_Polished (Game|GetPlayerCharacter 0)))
    (Variables|/Game/Blueprints/Players/Player_Polished.Player_Polished_C|SetTutorialActivated _asplayer_polished false)))

(fn ConstructionScript)