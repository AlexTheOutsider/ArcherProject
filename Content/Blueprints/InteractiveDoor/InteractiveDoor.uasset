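; Interactive sliding door that opens and closes by a timeline lerping the door's relative location between start and end points.
; A component tagged "Hand" entering the trigger volume either opens it automatically or, when Usable, enables the Interact input to toggle it.
; Each opening also notifies DoorCounter to increase its count.
; The construction script applies uniform frame scale and optional mesh and material overrides for door and frame.
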(event OnComponentBeginOverlap(TriggerVolume)
  (params (OverlappedComponent :type Primitive%20Component%20Object%20Reference) (OtherActor :type Actor%20Object%20Reference) (OtherComp :type Primitive%20Component%20Object%20Reference) (OtherBodyIndex :type Integer) (bFromSweep :type Boolean) (SweepResult :type Hit%20Result%20Structure%20%28by%20ref%29))
  (if (Components|ComponentHasTag OtherComp "Hand")
    (if (Variables|DoorSetup|GetUsable)
      (Input|EnableInput (Game|GetPlayerController 0))
      (else
        (CallFunction|DoorOpen)))))

(event OnComponentEndOverlap(TriggerVolume)
  (params (OverlappedComponent :type Primitive%20Component%20Object%20Reference) (OtherActor :type Actor%20Object%20Reference) (OtherComp :type Primitive%20Component%20Object%20Reference) (OtherBodyIndex :type Integer))
  (if (Components|ComponentHasTag OtherComp "Hand")
    (if (Variables|DoorSetup|GetUsable)
      (Input|DisableInput (Game|GetPlayerController 0))
      (else
        (CallFunction|DoorClose)))))

(event Custom|DoorOpen
  ;[1 1 1] Handles door motion for opening and closing.
  (Class|InterfaceInteractiveDoor|IncreaseDoorCount(Message) (Variables|DoorSetup|GetDoorCounter))
  (Variables|Mesh&MaterialOverride|SetIsOpened true)
  (bind _driver (Timeline|Timeline%20-%20Door%20Driver Play)
    (:Update
      (Transformation|SetRelativeLocation (Variables|Default|GetDoor) (Math|Vector|Lerp(Vector) (Variables|DoorSetup|GetDoorStart) (Variables|DoorSetup|GetDoorEnd) _driver) false false))))

(event Custom|DoorClose
  ;[1 1 1] Handles door motion for opening and closing.
  (Variables|Mesh&MaterialOverride|SetIsOpened false)
  (bind _driver (Timeline|Timeline%20-%20Door%20Driver Reverse)
    (:Update
      (Transformation|SetRelativeLocation (Variables|Default|GetDoor) (Math|Vector|Lerp(Vector) (Variables|DoorSetup|GetDoorStart) (Variables|DoorSetup|GetDoorEnd) _driver) false false))))

(event Input|ActionEvents|InputActionInteract
  (params (Key :type Key%20Structure :default "None"))
  (:Pressed
    (if (Variables|Mesh&MaterialOverride|GetIsOpened)
      (CallFunction|DoorClose)
      (else
        (CallFunction|DoorOpen)))))

(fn ConstructionScript
  (bind _3d_scale (Variables|DoorSetup|Get3D%20Scale))
  (Transformation|SetRelativeScale3D (Variables|Default|GetDoorFrame) (Math|Vector|MakeVector _3d_scale _3d_scale _3d_scale))
  (Utilities|FlowControl|Sequence
    (:then_0
      (|MeshOverride-Door))
    (:then_1
      (|MeshOverride-DoorFrame))
    (:then_2
      (|MaterialOverride-Door))
    (:then_3
      (|MaterialOverride-DoorFrame))))