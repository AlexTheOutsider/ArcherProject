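; Landed arrow that reports a noise on spawn and can be picked up by the player, breaking any attached rope and restoring ammo.
; Interact input turns on when the player's hand overlaps and a trace to the camera is unblocked, or remotely while hooked.
; The player's hook upgrade governs whether the hook trigger responds to its trace channel.
; The jump-over foothold collision logic is deprecated and disconnected.
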(event OnComponentBeginOverlap(InteractionTrigger)
  (params (OverlappedComponent :type Primitive%20Component%20Object%20Reference) (OtherActor :type Actor%20Object%20Reference) (OtherComp :type Primitive%20Component%20Object%20Reference) (OtherBodyIndex :type Integer) (bFromSweep :type Boolean) (SweepResult :type Hit%20Result%20Structure%20%28by%20ref%29))
  ;[1 1 1] Toggle Input
  (if (Components|ComponentHasTag OtherComp "Hand")
    (bind _visible (CallFunction|IsVisible))
    (if _visible
      (bind _asplayer_polished (Utilities|Casting|CastToPlayer_Polished (Game|GetPlayerCharacter 0)))
      (Variables|/Game/Blueprints/Players/Player_Polished.Player_Polished_C|SetInteractionInRange _asplayer_polished true)
      (Input|EnableInput (Game|GetPlayerController 0)))))

(event OnComponentEndOverlap(InteractionTrigger)
  (params (OverlappedComponent :type Primitive%20Component%20Object%20Reference) (OtherActor :type Actor%20Object%20Reference) (OtherComp :type Primitive%20Component%20Object%20Reference) (OtherBodyIndex :type Integer))
  ;[1 1 1] Toggle Input
  (if (and (Components|ComponentHasTag OtherComp "Hand") (not (Variables|Default|GetHooked)))
    (bind _asplayer_polished (Utilities|Casting|CastToPlayer_Polished (Game|GetPlayerCharacter 0)))
    (Variables|/Game/Blueprints/Players/Player_Polished.Player_Polished_C|SetInteractionInRange _asplayer_polished false)
    (Input|DisableInput (Game|GetPlayerController 0))))

(event OnComponentEndOverlap(JumpOverTrigger)
  (params (OverlappedComponent :type Primitive%20Component%20Object%20Reference) (OtherActor :type Actor%20Object%20Reference) (OtherComp :type Primitive%20Component%20Object%20Reference) (OtherBodyIndex :type Integer))
  ;[1 1 1] Deprecated: Set Foothold Collision to Overlap When Player is Moving Upward (conflicts with wall climbing since wall climbing doesn't override horizontal speed)
)

(event OnComponentBeginOverlap(JumpOverTrigger)
  (params (OverlappedComponent :type Primitive%20Component%20Object%20Reference) (OtherActor :type Actor%20Object%20Reference) (OtherComp :type Primitive%20Component%20Object%20Reference) (OtherBodyIndex :type Integer) (bFromSweep :type Boolean) (SweepResult :type Hit%20Result%20Structure%20%28by%20ref%29))
  ;[1 1 1] Deprecated: Set Foothold Collision to Overlap When Player is Moving Upward (conflicts with wall climbing since wall climbing doesn't override horizontal speed)
)

(event Custom|EnableRemoteRecollect
  ;[1 1 1] For retrieving arrows remotely
  (Variables|Default|SetHooked true)
  (bind _asplayer_polished (Utilities|Casting|CastToPlayer_Polished (Game|GetPlayerCharacter 0)))
  (Variables|/Game/Blueprints/Players/Player_Polished.Player_Polished_C|SetInteractionInRange _asplayer_polished true)
  (Input|EnableInput (Game|GetPlayerController 0)))

(event Custom|BreakHookEvent
  ;[1 1 1] For retrieving arrows remotely
  (Variables|Default|SetHooked false)
  (bind _asplayer_polished (Utilities|Casting|CastToPlayer_Polished (Game|GetPlayerCharacter 0)))
  (Variables|/Game/Blueprints/Players/Player_Polished.Player_Polished_C|SetInteractionInRange _asplayer_polished false)
  (Input|DisableInput (Game|GetPlayerController 0)))

(event Custom|HookUpgrade
  ;[1 1 1] Hook Upgrade
  (bind _asplayer_polished (Utilities|Casting|CastToPlayer_Polished (Game|GetPlayerCharacter 0)))
  (if (Variables|/Game/Blueprints/Players/Player_Polished.Player_Polished_C|GetHookArrowUpgrade _asplayer_polished) ; not necessary, just in case
    (if (Variables|Default|GetAttached)
      (Collision|SetCollisionResponsetoChannel (Variables|Default|GetHookTrigger) "ECC_GameTraceChannel2" "ECR_Overlap"))))

(event EventBeginPlay
  ;[1 1 1] Initialization (including making noise)
  (Rendering|SetVisibility (Variables|Default|GetWidget) false false)
  (Class|AISenseHearing|ReportNoiseEvent (Transformation|GetActorLocation) 1.0 self 0.0 "Arrow Hit")
  (if (Variables|Default|GetIsAttachedToSwitch)
    _
    (else
      _))
  (bind _asplayer_polished (Utilities|Casting|CastToPlayer_Polished (Game|GetPlayerCharacter 0)))
  (if (not (Variables|/Game/Blueprints/Players/Player_Polished.Player_Polished_C|GetHookArrowUpgrade _asplayer_polished))
    (Collision|SetCollisionResponsetoChannel (Variables|Default|GetHookTrigger) "ECC_GameTraceChannel2" "ECR_Ignore")))

(event Input|ActionEvents|InputActionInteract
  (params (Key :type Key%20Structure :default "None"))
  (bind _self self)
  ;[1 1 1] Recollect Arrow
  (:Pressed
    (bind _asplayer_polished (Utilities|Casting|CastToPlayer_Polished (Game|GetPlayerCharacter 0)))
    (Default|BreakRopeforRecollectingActivatedHookPoint _asplayer_polished _self)
    (Utilities|Array|RemoveItem (Variables|/Game/Blueprints/Players/Player_Polished.Player_Polished_C|GetStaticArrowArray _asplayer_polished) _self)
    (Default|ResumeArrowAmount _asplayer_polished)
    (bind _asplayer_polished_2 (Utilities|Casting|CastToPlayer_Polished (Game|GetPlayerCharacter 0)))
    (Variables|/Game/Blueprints/Players/Player_Polished.Player_Polished_C|SetInteractionInRange _asplayer_polished_2 false) ; actually redundant
    (Actor|DestroyActor)))

(fn ConstructionScript)

(fn IsVisible
  (bind _asplayer_polished (Utilities|Casting|CastToPlayer_Polished (Game|GetPlayerCharacter 0)))
  (bind _returnvalue (Collision|LineTraceByChannel (Transformation|GetWorldLocation (Variables|Default|GetVisiblePoint)) (Transformation|GetWorldLocation (Variables|/Game/Blueprints/Players/Player_Polished.Player_Polished_C|GetCamera _asplayer_polished)) "TraceTypeQuery1" false (Variables|Default|GetVisibilityIgnore) "None")) ; Pawn ignores visibility trace, but environments block it
  (return (not _returnvalue)))