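; Static arrow actor that cannot be recollected, apparently a stripped-down variant of a recollectable arrow that served as a foothold.
; On BeginPlay it hides its widget and reports an "Arrow Hit" noise event at its own location.
; Trigger overlap events are empty, leaving the recollect, input-toggle and deprecated jump-through collision logic disconnected and never run.
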(event OnComponentBeginOverlap(InteractionTrigger_0)
  (params (OverlappedComponent :type Primitive%20Component%20Object%20Reference) (OtherActor :type Actor%20Object%20Reference) (OtherComp :type Primitive%20Component%20Object%20Reference) (OtherBodyIndex :type Integer) (bFromSweep :type Boolean) (SweepResult :type Hit%20Result%20Structure%20%28by%20ref%29))
  ;[1 1 1] Toggle Input
)

(event OnComponentEndOverlap(InteractionTrigger_0)
  (params (OverlappedComponent :type Primitive%20Component%20Object%20Reference) (OtherActor :type Actor%20Object%20Reference) (OtherComp :type Primitive%20Component%20Object%20Reference) (OtherBodyIndex :type Integer))
  ;[1 1 1] Toggle Input
)

(event OnComponentEndOverlap(JumpOverTrigger_0)
  (params (OverlappedComponent :type Primitive%20Component%20Object%20Reference) (OtherActor :type Actor%20Object%20Reference) (OtherComp :type Primitive%20Component%20Object%20Reference) (OtherBodyIndex :type Integer))
  ;[1 1 1] Deprecated: Set Foothold Collision to Overlap When Player is Moving Upward (conflicts with wall climbing since wall climbing doesn't override horizontal speed)
)

(event OnComponentBeginOverlap(JumpOverTrigger_0)
  (params (OverlappedComponent :type Primitive%20Component%20Object%20Reference) (OtherActor :type Actor%20Object%20Reference) (OtherComp :type Primitive%20Component%20Object%20Reference) (OtherBodyIndex :type Integer) (bFromSweep :type Boolean) (SweepResult :type Hit%20Result%20Structure%20%28by%20ref%29))
  ;[1 1 1] Deprecated: Set Foothold Collision to Overlap When Player is Moving Upward (conflicts with wall climbing since wall climbing doesn't override horizontal speed)
)

(event EventBeginPlay
  ;[1 1 1] Initialization
  (Rendering|SetVisibility (Variables|Default|GetWidget) false false)
  (Class|AISenseHearing|ReportNoiseEvent (Transformation|GetActorLocation) 1.0 self 0.0 "Arrow Hit"))

(event Input|ActionEvents|InputActionInteract
  (params (Key :type Key%20Structure :default "None"))
  ;[1 1 1] Recollect Arrow
)

(fn ConstructionScript)