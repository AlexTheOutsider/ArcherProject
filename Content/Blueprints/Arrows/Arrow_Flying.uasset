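; Flying arrow projectile that takes its speed limits from Player_Polished and raises gravity each tick as it slows.
; On its first non-player overlap it sphere-traces along the shaft, swaps itself for an attached Arrow_Static tracked by the player, and spawns blood or dust.
; A failed trace or projectile stop destroys it and calls ResumeArrowAmount on the player.
; Hit events damage "Breakable" actors; air friction and manual rotation are deprecated.
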(event OnProjectileStop(ProjectileMovement)
  (params (ImpactResult :type Hit%20Result%20Structure%20%28by%20ref%29))
  ;[1 1 1] On Stop
  (Utilities|FlowControl|Delay 1.0)
  (bind _asplayer_polished (Utilities|Casting|CastToPlayer_Polished (Game|GetPlayerCharacter 0)))
  (Default|ResumeArrowAmount _asplayer_polished)
  (Actor|DestroyActor))

(event Custom|ArrowAngle
  (bind _returnvalue (Transformation|GetActorRotation))
  ;[1 1 1] Deprecated: Arrow Angle (use build-in function instead)
  (Transformation|SetActorRotation (Math|Rotator|MakeRotator (.roll _returnvalue) (.pitch (Math|Rotator|MakeRotfromX (Transformation|GetVelocity))) (.yaw _returnvalue))))

(event Custom|AdjustGravityScale
  ;[1 1 1] Adjust Gravity Scale
  (Utilities|Casting|CastToPlayer_Polished (Game|GetPlayerCharacter 0))
  (Variables|/Script/Engine.ProjectileMovementComponent|SetProjectileGravityScale (Variables|Default|GetProjectileMovement) (* (- 1.0 (/ (- (Math|Vector|VectorLength (Transformation|GetVelocity)) (Variables|General|GetMinSpeed)) (- (Variables|General|GetMaxSpeed) (Variables|General|GetMinSpeed)))) (Variables|General|GetGravityScale))))

(event EventBeginPlay
  ;[1 1 1] Initialization
  (|InitialSetup))

(event Collision|EventHit
  (params (MyComp :type Primitive%20Component%20Object%20Reference) (Other :type Actor%20Object%20Reference) (OtherComp :type Primitive%20Component%20Object%20Reference) (bSelfMoved :type Boolean) (HitLocation :type Vector :default "0, 0, 0") (HitNormal :type Vector :default "0, 0, 0") (NormalImpulse :type Vector :default "0, 0, 0") (Hit :type Hit%20Result%20Structure%20%28by%20ref%29))
  ;[1 1 1] Break Glass
  (if (Actor|ActorHasTag Other "Breakable")
    (Game|Damage|ApplyPointDamage Other 1e+02 HitLocation Hit 0 0 "/Script/Engine.DamageType")))

(event Collision|EventActorBeginOverlap
  (params (OtherActor :type Actor%20Object%20Reference))
  ;[1 1 1] On Landed
  (if (not (Actor|ActorHasTag OtherActor "Player"))
    (if (Variables|OnLanded|GetDoOnce)
      (Variables|OnLanded|SetDoOnce false)
      (bind (_outhit _returnvalue) (Collision|SphereTraceByChannel (Transformation|GetWorldLocation (Variables|Default|GetArrowEnd)) (Transformation|GetWorldLocation (Variables|Default|GetArrowStart)) (Variables|General|GetArrowRadius) "TraceTypeQuery6" false 0 "None"))
      (Development|PrintString (Utilities|String|Append "Arrow Hit: 
" (Utilities|GetDisplayName (.hitcomponent _outhit)) " 
Overlap: 
" (Utilities|GetDisplayName OtherActor)) false)
      (if _returnvalue
        (Variables|OnLanded|SetHitActor (.hitactor _outhit))
        (Variables|OnLanded|SetHitLocation (.location _outhit))
        (Variables|OnLanded|SetHitComponent (.hitcomponent _outhit))
        (if (Utilities|Name|Equal(Name) (.hitbonename _outhit) "None")
          _
          (else
            _))
        (Components|Movement|StopMovementImmediately (Variables|Default|GetProjectileMovement))
        (Transformation|SetActorLocation (Variables|OnLanded|GetHitLocation) false false)
        ;[1 1 1] Generate Static Arrow
        (bind _returnvalue_2 (Game|SpawnActorfromClass "/Game/Blueprints/Arrows/Arrow_Static.Arrow_Static_C" (Transformation|GetActorTransform) "Undefined" 0 0))
        (bind _asplayer_polished (Utilities|Casting|CastToPlayer_Polished (Game|GetPlayerCharacter 0)))
        (Utilities|Array|Add (Variables|/Game/Blueprints/Players/Player_Polished.Player_Polished_C|GetStaticArrowArray _asplayer_polished) _returnvalue_2)
        (Transformation|AttachComponentToComponent _returnvalue_2 (Variables|OnLanded|GetHitComponent) (.hitbonename _outhit) "KeepWorld" "KeepWorld" "KeepWorld" true)
        (switch Utilities|FlowControl|Switch|SwitchonECollisionChannel (Collision|GetCollisionObjectType (Variables|OnLanded|GetHitComponent))
          (:ECC_WorldStatic
            (Effects|SpawnEmitteratLocation "/Game/Textures/Particles/Dust.Dust" (Variables|OnLanded|GetHitLocation) :!label _label))
          (:ECC_WorldDynamic
            (goto _label))
          (:ECC_Pawn
            (Effects|SpawnEmitteratLocation "/Game/Textures/Particles/Blood.Blood" (Variables|OnLanded|GetHitLocation)))
          (:ECC_PhysicsBody
            (goto _label))
          (:ECC_Vehicle
            (goto _label))
          (:ECC_Destructible
            (goto _label)))
        (Actor|DestroyActor)
        (else
          (Actor|DestroyActor) ; If arrow hits anything else that overlaps with it, destroy itself.
          (bind _asplayer_polished_2 (Utilities|Casting|CastToPlayer_Polished (Game|GetPlayerCharacter 0)))
          (Default|ResumeArrowAmount _asplayer_polished_2))))))

(event EventTick
  (params (DeltaSeconds :type Float%20%28single-precision%29))
  ;[1 1 1] Event Tick
  (CallFunction|AdjustGravityScale))

(fn ConstructionScript)