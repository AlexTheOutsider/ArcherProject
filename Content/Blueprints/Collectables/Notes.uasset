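; A collectable note that the player can read, built on a parent interactable class whose overlap handling it overrides.
; A "Hand"-tagged component entering the trigger enables input and flags interaction range on Player_Polished, unless the note is Invalid.
; Interact toggles the player's reading state, passes over the note's title and texts, and recolours the Cube.
; Leaving the trigger or EndPickUp clears both flags and disables input.
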(event OnComponentBeginOverlap(InteractionTrigger)
  (params (OverlappedComponent :type Primitive%20Component%20Object%20Reference) (OtherActor :type Actor%20Object%20Reference) (OtherComp :type Primitive%20Component%20Object%20Reference) (OtherBodyIndex :type Integer) (bFromSweep :type Boolean) (SweepResult :type Hit%20Result%20Structure%20%28by%20ref%29))
  ;[1 1 1] Toggle Input (override parent's function)
  (if (Components|ComponentHasTag OtherComp "Hand")
    (if (not (Variables|Default|GetInvalid))
      (bind _asplayer_polished (Utilities|Casting|CastToPlayer_Polished (Game|GetPlayerCharacter 0)))
      (Variables|/Game/Blueprints/Players/Player_Polished.Player_Polished_C|SetInteractionInRange _asplayer_polished true)
      (Input|EnableInput (Game|GetPlayerController 0)))))

(event OnComponentEndOverlap(InteractionTrigger)
  (params (OverlappedComponent :type Primitive%20Component%20Object%20Reference) (OtherActor :type Actor%20Object%20Reference) (OtherComp :type Primitive%20Component%20Object%20Reference) (OtherBodyIndex :type Integer))
  ;[1 1 1] Toggle Input (override parent's function)
  (if (Components|ComponentHasTag OtherComp "Hand")
    (bind _asplayer_polished (Utilities|Casting|CastToPlayer_Polished (Game|GetPlayerCharacter 0)))
    (Variables|/Game/Blueprints/Players/Player_Polished.Player_Polished_C|SetInteractionInRange _asplayer_polished false)
    (Variables|/Game/Blueprints/Players/Player_Polished.Player_Polished_C|SetIsReading _asplayer_polished false)
    (Input|DisableInput (Game|GetPlayerController 0))))

(event EventBeginPlay
  (|CallParentFunction))

(event EventEndPickUp
  ;[1 1 1] Toggle Input (override parent's function)
  (bind _asplayer_polished (Utilities|Casting|CastToPlayer_Polished (Game|GetPlayerCharacter 0)))
  (Variables|/Game/Blueprints/Players/Player_Polished.Player_Polished_C|SetInteractionInRange _asplayer_polished false)
  (Variables|/Game/Blueprints/Players/Player_Polished.Player_Polished_C|SetIsReading _asplayer_polished false)
  (Input|DisableInput (Game|GetPlayerController 0)))

(event EventTick
  (params (DeltaSeconds :type Float%20%28single-precision%29))
  (|CallParentFunction DeltaSeconds))

(event Input|ActionEvents|InputActionInteract
  (params (Key :type Key%20Structure :default "None"))
  (:Pressed
    (bind _asplayer_polished (Utilities|Casting|CastToPlayer_Polished (Game|GetPlayerCharacter 0)))
    (Variables|/Game/Blueprints/Players/Player_Polished.Player_Polished_C|SetIsReading _asplayer_polished (not (Variables|/Game/Blueprints/Players/Player_Polished.Player_Polished_C|GetIsReading _asplayer_polished)))
    (Variables|/Game/Blueprints/Players/Player_Polished.Player_Polished_C|SetNoteTitle _asplayer_polished (Variables|Default|GetTitle))
    (Variables|/Game/Blueprints/Players/Player_Polished.Player_Polished_C|SetNoteTexts _asplayer_polished (Variables|Default|GetTexts))
    (Rendering|Material|SetMaterial (Variables|Default|GetCube) 1 "/Game/Geometry/Blockmesh/meshblock_colored/Materials/0071_MediumSpringGreen.0071_MediumSpringGreen")))

(fn ConstructionScript)