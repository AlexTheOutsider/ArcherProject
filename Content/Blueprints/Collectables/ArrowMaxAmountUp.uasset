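; Collectable pickup that permanently raises the player's maximum arrow capacity.
; It extends a parent collectable, binding PickUp to its pickup event, which adds UpAmount to both max and current arrows on Player_Polished.
; Pickup also prints a debug message, recolors the cube, and passes a skill title, description and unlocked flag to the player.
; The tutorial text unlock call is marked deprecated but still runs.
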(event Custom|PickUp
  (bind _upamount (Variables|Default|GetUpAmount))
  (bind _asplayer_polished (Utilities|Casting|CastToPlayer_Polished (Game|GetPlayerCharacter 0)))
  (Variables|/Game/Blueprints/Players/Player_Polished.Player_Polished_C|SetArrowMaxAmount _asplayer_polished (+ (Variables|/Game/Blueprints/Players/Player_Polished.Player_Polished_C|GetArrowMaxAmount _asplayer_polished) _upamount))
  (Variables|/Game/Blueprints/Players/Player_Polished.Player_Polished_C|SetArrowAmount _asplayer_polished (+ (Variables|/Game/Blueprints/Players/Player_Polished.Player_Polished_C|GetArrowAmount _asplayer_polished) _upamount))
  (Development|PrintString "Max arrow amount has been increased!")
  (CallFunction|UnlockTutorialText) ; Deprecated.
  (Rendering|Material|SetMaterial (Variables|Default|GetCube) 1 "/Game/Geometry/Blockmesh/meshblock_colored/Materials/0071_MediumSpringGreen.0071_MediumSpringGreen")
  (Variables|/Game/Blueprints/Players/Player_Polished.Player_Polished_C|SetSkillTitle _asplayer_polished (Variables|Default|GetSkillName))
  (Variables|/Game/Blueprints/Players/Player_Polished.Player_Polished_C|SetSkillDescription _asplayer_polished (Variables|Default|GetSkillDescription))
  (Variables|/Game/Blueprints/Players/Player_Polished.Player_Polished_C|SetSkillUnlocked _asplayer_polished true))

(event EventBeginPlay
  (|CallParentFunction)
  (EventDispatchers|BindEventtoOnPickUp (delegate Custom|PickUp)))

(event EventTick
  (params (DeltaSeconds :type Float%20%28single-precision%29))
  (|CallParentFunction DeltaSeconds))

(fn ConstructionScript
  (Variables|Default|SetTutorialText "Pick up bow to shoot arrows")
  (|CallParentFunction))