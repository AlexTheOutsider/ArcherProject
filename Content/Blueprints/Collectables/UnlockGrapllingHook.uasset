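; A collectable pickup that unlocks the grappling hook ability for the player, built on a parent class.
; Its construction script sets the tutorial text and row name before running the parent construction.
; On the OnPickUp event it sets the unlock flag on Player_Polished, calls UnlockTutorialText and recolors its cube green.
; It also copies the skill name and description to the player and flags a skill as unlocked.
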(event Custom|PickUp
  (bind _asplayer_polished (Utilities|Casting|CastToPlayer_Polished (Game|GetPlayerCharacter 0)))
  (Variables|/Game/Blueprints/Players/Player_Polished.Player_Polished_C|SetUnlockGrapplingHook _asplayer_polished true)
  (Development|PrintString "Grappling Hook Unlocked!" false true "(R=0.000000,G=0.660000,B=1.000000,A=1.000000)" 1e+01)
  (CallFunction|UnlockTutorialText)
  (Rendering|Material|SetMaterial (Variables|Default|GetCube) 0 "/Game/Geometry/Blockmesh/meshblock_colored/Materials/0071_MediumSpringGreen.0071_MediumSpringGreen")
  (Variables|/Game/Blueprints/Players/Player_Polished.Player_Polished_C|SetSkillName _asplayer_polished (Variables|Default|GetSkillName))
  (Variables|/Game/Blueprints/Players/Player_Polished.Player_Polished_C|SetSkillDescription _asplayer_polished (Variables|Default|GetSkillDescription))
  (Variables|/Game/Blueprints/Players/Player_Polished.Player_Polished_C|SetSkillUnlocked _asplayer_polished true))

(event EventBeginPlay
  (|CallParentFunction)
  (EventDispatchers|BindEventtoOnPickUp (delegate Custom|PickUp)))

(event EventTick
  (params (DeltaSeconds :type Float%20%28single-precision%29))
  (|CallParentFunction DeltaSeconds))

(fn ConstructionScript
  (Variables|Default|SetTutorialText "Pick up grapplng hook to fast travel")
  (Variables|Default|SetRowName "UnlockGrapllingHook")
  (|CallParentFunction))