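; ArrowAmountUp is a collectable pickup that raises the player's arrow capacity.
; Each tick it spins its widget component around yaw by RotationSpeed.
; When a component tagged "Body" on a Player_Polished overlaps its trigger, it adds UpAmount to both the player's maximum and current arrows, then destroys itself.
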(event OnComponentBeginOverlap(AutomaticTrigger)
  (params (OverlappedComponent :type Primitive%20Component%20Object%20Reference) (OtherActor :type Actor%20Object%20Reference) (OtherComp :type Primitive%20Component%20Object%20Reference) (OtherBodyIndex :type Integer) (bFromSweep :type Boolean) (SweepResult :type Hit%20Result%20Structure%20%28by%20ref%29))
  (bind _upamount (Variables|Default|GetUpAmount))
  (if (Components|ComponentHasTag OtherComp "Body")
    (bind _asplayer_polished (Utilities|Casting|CastToPlayer_Polished OtherActor))
    (Variables|/Game/Blueprints/Characters/Players/Player_Polished.Player_Polished_C|SetArrowMaxAmount _asplayer_polished (+ (Variables|/Game/Blueprints/Characters/Players/Player_Polished.Player_Polished_C|GetArrowMaxAmount _asplayer_polished) _upamount))
    (Variables|/Game/Blueprints/Characters/Players/Player_Polished.Player_Polished_C|SetArrowAmount _asplayer_polished (+ (Variables|/Game/Blueprints/Characters/Players/Player_Polished.Player_Polished_C|GetArrowAmount _asplayer_polished) _upamount))
    (Actor|DestroyActor)))

(event EventTick
  (params (DeltaSeconds :type Float%20%28single-precision%29))
  (bind _widget (Variables|Default|GetWidget))
  (bind _returnvalue (Transformation|GetWorldRotation _widget))
  (Transformation|SetWorldRotation _widget (Math|Rotator|MakeRotator (.roll _returnvalue) (.pitch _returnvalue) (+ (.yaw _returnvalue) (Variables|Default|GetRotationSpeed))) false false))

(fn ConstructionScript)