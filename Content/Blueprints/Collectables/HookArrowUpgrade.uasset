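; HookArrowUpgrade is a collectable that upgrades the player's grappling hook so it can hook onto the ends of arrows.
; When a component tagged Body overlaps its trigger and belongs to Player_Polished, it sets the player's HookArrowUpgrade flag.
; It then calls HookUpgrade on every arrow in the player's StaticArrowArray, prints an on-screen notice and destroys itself.
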(event OnComponentBeginOverlap(AutomaticTrigger)
  (params (OverlappedComponent :type Primitive%20Component%20Object%20Reference) (OtherActor :type Actor%20Object%20Reference) (OtherComp :type Primitive%20Component%20Object%20Reference) (OtherBodyIndex :type Integer) (bFromSweep :type Boolean) (SweepResult :type Hit%20Result%20Structure%20%28by%20ref%29))
  (if (Components|ComponentHasTag OtherComp "Body")
    (bind _asplayer_polished (Utilities|Casting|CastToPlayer_Polished OtherActor))
    (Variables|/Game/Blueprints/Players/Player_Polished.Player_Polished_C|SetHookArrowUpgrade _asplayer_polished true)
    (for _array_element (Variables|/Game/Blueprints/Players/Player_Polished.Player_Polished_C|GetStaticArrowArray _asplayer_polished)
      (Default|HookUpgrade _array_element))
    (Development|PrintString "Grappling Hook Upgraded! Now you can hook on arrows' end!" true true "(R=0.000000,G=0.660000,B=1.000000,A=1.000000)" 1e+01)
    (Actor|DestroyActor)))

(event EventTick
  (params (DeltaSeconds :type Float%20%28single-precision%29))
  (|CallParentFunction DeltaSeconds))

(fn ConstructionScript)