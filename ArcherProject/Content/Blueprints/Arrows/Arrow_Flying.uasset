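; Arrow projectile actor that pitches along its velocity in flight and sticks into what it hits.
; On its first overlap only, it line traces forward from its Sphere, with debug drawing, to find the hit point, component and bone.
; A successful trace swaps it for an Arrow_Static attached there, spawns blood for pawns and physics bodies or dust for other surfaces, then destroys itself.
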(event Custom|ArrowAngle
  (bind _returnvalue (Transformation|GetActorRotation))
  (Transformation|SetActorRotation (Math|Rotator|MakeRotator (.roll _returnvalue) (.pitch (Math|Rotator|MakeRotfromX (Transformation|GetVelocity))) (.yaw _returnvalue))))

(event Collision|EventActorBeginOverlap
  (params (OtherActor :type Actor%20Object%20Reference))
  (bind _sphere (Variables|Default|GetSphere))
  (bind _returnvalue (Transformation|GetWorldLocation _sphere))
  (if (Variables|Default|GetDoOnce)
    (Variables|Default|SetDoOnce false)
    (bind (_outhit _returnvalue_2) (Collision|LineTraceByChannel _returnvalue (+ _returnvalue (* (Math|Vector|GetForwardVector (Transformation|GetWorldRotation _sphere)) 2e+02)) "TraceTypeQuery1" false 0 "ForDuration"))
    (Development|PrintString (Utilities|String|Append "Arrow Hit: " (Utilities|GetDisplayName (.hitcomponent _outhit))) false)
    (if _returnvalue_2
      (Variables|HitResult|SetHitActor (.hitactor _outhit))
      (Variables|HitResult|SetHitLocation (.location _outhit))
      (Variables|HitResult|SetHitComponent (.hitcomponent _outhit))
      (if (Utilities|Name|Equal(Name) (.hitbonename _outhit) "None")
        _
        (else
          _))
      (Components|Movement|StopMovementImmediately (Variables|Default|GetProjectileMovement))
      (Transformation|SetActorLocation (Variables|HitResult|GetHitLocation) false false)
      (bind _returnvalue_3 (Game|SpawnActorfromClass "/Game/Blueprints/Arrows/Arrow_Static.Arrow_Static_C" (Transformation|GetActorTransform) "Undefined" 0 0))
      (Transformation|AttachComponentToComponent _returnvalue_3 (Variables|HitResult|GetHitComponent) (.hitbonename _outhit) "KeepWorld" "KeepWorld" "KeepWorld" true)
      (switch Utilities|FlowControl|Switch|SwitchonECollisionChannel (Collision|GetCollisionObjectType (Variables|HitResult|GetHitComponent))
        (:ECC_WorldStatic
          (Effects|SpawnEmitteratLocation "/Game/Textures/Particles/Dust.Dust" (Variables|HitResult|GetHitLocation) :!label _label))
        (:ECC_WorldDynamic
          (goto _label))
        (:ECC_Pawn
          (Effects|SpawnEmitteratLocation "/Game/Textures/Particles/Blood.Blood" (Variables|HitResult|GetHitLocation) :!label _label_2))
        (:ECC_PhysicsBody
          (goto _label_2))
        (:ECC_Vehicle
          (goto _label))
        (:ECC_Destructible
          (goto _label)))
      (Actor|DestroyActor))))

(event EventTick
  (params (DeltaSeconds :type Float%20%28single-precision%29))
  (if (not (Math|Vector|Equal(Vector) (Variables|/Script/Engine.MovementComponent|GetVelocity (Variables|Default|GetProjectileMovement)) "0, 0, 0" 0.0001))
    (CallFunction|ArrowAngle)))

(fn ConstructionScript)