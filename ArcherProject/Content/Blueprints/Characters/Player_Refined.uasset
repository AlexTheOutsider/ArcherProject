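; Player character with air jump, camera-directed dash, timed wall climbing, grapple hook and charged arrow shot.
; Tick updates the idle state that gates dash and fire, drives climbing on "Climbable"-tagged walls, and constrains hooked movement with a counter-force beyond rope length.
; The grapple traces from the camera and animates a cable via timelines; pressing again launches toward the hook, while jump breaks the rope.
; Landing resets air jump and climb.
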(event Custom|ResetAirJump
  ;[1 1 1] Air Jump
  (Variables|AirJump|SetCanAirJump true))

(event EventOnLanded
  (params (Hit :type Hit%20Result%20Structure%20%28by%20ref%29))
  ;[1 1 1] Event On Landed
  (CallFunction|ResetAirJump)
  (CallFunction|ResetClimb))

(event EventBeginPlay
  ;[1 1 1] Initialization
  (Variables|/Script/Engine.CharacterMovementComponent|SetAirControl (Variables|Character|GetCharacterMovement) (Variables|Default|GetDefaultAirControl)))

(event EventTick
  (params (DeltaSeconds :type Float%20%28single-precision%29))
  ;[1 1 1] Event Tick
  (Variables|Default|SetDeltaTime DeltaSeconds)
  (Utilities|FlowControl|Sequence
    (:then_0
      (|SetIsIdle))
    (:then_1
      (|Climb))
    (:then_2
      (|Hooked))))

(event Input|ActionEvents|InputActionJump
  (params (Key :type Key%20Structure))
  ;[1 1 1] Air Jump
  (:Pressed
    (Variables|Climb|SetIsJumpKeyPressed true)
    (if (Variables|GrappleHook|GetGrappleHooked)
      (CallFunction|BreakGrappleRope))
    (bind _newparam (CallFunction|GroundCheck))
    (if _newparam
      (Character|Jump)
      (elif (Variables|AirJump|GetCanAirJump)
        (Variables|AirJump|SetCanAirJump false)
        (Character|LaunchCharacter (Math|Vector|MakeVector 0.0 0.0 (Variables|AirJump|GetAirJumpSpeed)) false true))))
  (:Released
    (Variables|Climb|SetIsJumpKeyPressed false)))

(event Input|ActionEvents|InputActionDash
  (params (Key :type Key%20Structure))
  ;[1 1 1] Dash
  (:Pressed
    (if (Variables|Dash|GetCanDash)
      (if (Variables|Default|GetIsIdle)
        (Character|LaunchCharacter (* (Math|Vector|GetForwardVector (Variables|Default|GetCamera)) (Variables|Dash|GetDashDistance)) true true)
        (Variables|Dash|SetCanDash false)
        (Utilities|FlowControl|Delay 0.03) ; If there is no deday, character will keep moving and won't be stopped by the next node
        (Components|Movement|StopMovementImmediately (Variables|Character|GetCharacterMovement))
        (Utilities|FlowControl|Delay (Variables|Dash|GetDashCooldown))
        (Variables|Dash|SetCanDash true)))))

(event Input|ActionEvents|InputActionGrappleHook
  (params (Key :type Key%20Structure))
  ;[1 1 1] GrappleHook
  (:Pressed
    (|GrappleHook)))

(event Input|ActionEvents|InputActionFire
  (params (Key :type Key%20Structure))
  ;[1 1 1] Shoot Arrow
  (:Pressed
    (if (Variables|Default|GetIsIdle)
      (|ShootArrow :!label _label)))
  (:Released
    (if (Variables|Arrow|GetHoldFire)
      (goto _label Released))))

(event Input|AxisEvents|InputAxisMouseLookHorizontal
  (params (AxisValue :type Float%20%28single-precision%29))
  ;[1 1 1] Character Orientation
  (Pawn|Input|AddControllerYawInput AxisValue))

(event Input|AxisEvents|InputAxisMouseLookVertical
  (params (AxisValue :type Float%20%28single-precision%29))
  ;[1 1 1] Character Orientation
  (Pawn|Input|AddControllerPitchInput AxisValue))

(event Input|AxisEvents|InputAxisHorizontalMovement
  (params (AxisValue :type Float%20%28single-precision%29))
  ;[1 1 1] Character Movement
  (if (|IsNotActuallyClimbing)
    (Pawn|Input|AddMovementInput (Math|Vector|GetRightVector (Math|Rotator|MakeRotator 0.0 0.0 (.yaw (Pawn|GetControlRotation :!class /Script/Engine.Pawn)))) AxisValue false)))

(event Input|AxisEvents|InputAxisVerticalMovement
  (params (AxisValue :type Float%20%28single-precision%29))
  ;[1 1 1] Character Movement
  (Pawn|Input|AddMovementInput (Math|Vector|GetForwardVector (Math|Rotator|MakeRotator 0.0 0.0 (.yaw (Pawn|GetControlRotation :!class /Script/Engine.Pawn)))) AxisValue false)
  (if (> AxisValue 0.0)
    (Variables|Climb|SetIsMovingForward true)
    (else
      (Variables|Climb|SetIsMovingForward false))))

(fn ConstructionScript)

(fn GroundCheck
  (bind (_outhit _returnvalue) (Collision|LineTraceByChannel (Transformation|GetActorLocation) (Transformation|GetWorldLocation (Variables|Default|GetGroundHitLocation)) "TraceTypeQuery1" false 0 "None"))
  (if _returnvalue
    (if (Utilities|Enum|Equal(Enum) (Collision|GetCollisionObjectType (.hitcomponent _outhit)) "ECC_WorldStatic")
      (LocalVariables|SetReturnValue true)))
  (return (LocalVariables|GetReturnValue)))

(event OnComponentHit(CapsuleComponent)
  (params (HitComponent :type Primitive%20Component%20Object%20Reference) (OtherActor :type Actor%20Object%20Reference) (OtherComp :type Primitive%20Component%20Object%20Reference) (NormalImpulse :type Vector :default "0, 0, 0") (Hit :type Hit%20Result%20Structure%20%28by%20ref%29))
  ;[1 1 1] Deprecated: Extra Jump At the End of Grapple
)

(event Custom|ShootGrappleHookAnimation
  (bind _grapplerope (Variables|Default|GetGrappleRope))
  (bind _grapplerope_2 (Variables|Default|GetGrappleRope))
  ;[1 1 1] Shoot Grapple Hook Animation
  (Rendering|SetVisibility _grapplerope true false)
  (if (Variables|GrappleHook|GetGrappleHookHit)
    (Class|CableComponent|SetAttachEndto _grapplerope (Variables|GrappleHook|GetGrappleHookActor) "None" "None")
    (bind _curve (Timeline|Timeline%20-%20Shoot%20Grapple%20Hook PlayFromStart) ; It takes 0.3s for grapple hook to reach its end
      (:Update
        (|UpdateRopeEndLocation _curve))
      (:Finished
        (Variables|/Script/CableComponent.CableComponent|SetCableLength _grapplerope_2 (Variables|GrappleHook|GetGrappleRopeLength))
        (Variables|GrappleHook|SetIsGrappleHooking false)
        (if (Variables|GrappleHook|GetGrappleHookHit)
          (Variables|GrappleHook|SetGrappleHooked true)
          (else
            (Variables|/Script/CableComponent.CableComponent|SetbAttachEnd _grapplerope_2 false)
            (CallFunction|ContractGrappleRopeAnimation)))))
    (else
      (Timeline|Timeline%20-%20Shoot%20Grapple%20Hook PlayFromStart))))

(event Custom|ResetGrappleHook
  (bind _grapplerope (Variables|Default|GetGrappleRope))
  ;[1 1 1] Reset Grapple Hook
  (Variables|/Script/Engine.CharacterMovementComponent|SetAirControl (Variables|Character|GetCharacterMovement) (Variables|Default|GetDefaultAirControl))
  (Class|CableComponent|SetAttachEndto _grapplerope 0 "None" "None")
  (Variables|/Script/CableComponent.CableComponent|SetEndLocation _grapplerope "0, 0, 0")
  (Variables|/Script/CableComponent.CableComponent|SetbAttachEnd _grapplerope true)
  (Variables|GrappleHook|SetGrappleRopeLength 0.0)
  (Utilities|FlowControl|Delay (Variables|GrappleHook|GetGrappleHookCooldown))
  (Variables|GrappleHook|SetCanGrappleHook true))

(event Custom|BreakGrappleRope
  ;[1 1 1] Break Grapple Hook
  (Variables|GrappleHook|SetGrappleHooked false)
  (Variables|/Script/CableComponent.CableComponent|SetbAttachEnd (Variables|Default|GetGrappleRope) false)
  (CallFunction|ContractGrappleRopeAnimation))

(event Custom|ShootGrappleHook
  (bind _camera (Variables|Default|GetCamera))
  (bind _returnvalue (Transformation|GetWorldLocation _camera))
  ;[1 1 1] Check for Surface
  (if (Variables|GrappleHook|GetCanGrappleHook)
    (Variables|GrappleHook|SetCanGrappleHook false)
    (Variables|GrappleHook|SetIsGrappleHooking true)
    (bind _output_get (Variables|GrappleHook|SetGrappleHookLocation (+ _returnvalue (* (Math|Vector|GetForwardVector _camera) (Variables|GrappleHook|GetGrappleHookRange)))))
    (bind (_outhit _returnvalue_2) (Collision|LineTraceByChannel _returnvalue _output_get "TraceTypeQuery3" false 0 "ForDuration"))
    ;[1 1 1] Store Rope Information
    (bind _output_get_2 (Variables|GrappleHook|SetGrappleHookHit _returnvalue_2))
    (Variables|GrappleHook|SetGrappleHookActor (.hitactor _outhit))
    (if _output_get_2
      (Variables|GrappleHook|SetGrappleHookLocation (.location _outhit))
      (Variables|GrappleHook|SetGrappleRopeLength (.distance _outhit))
      (else
        (Variables|GrappleHook|SetGrappleRopeLength (Variables|GrappleHook|GetGrappleHookRange))))
    (CallFunction|ShootGrappleHookAnimation)))

(event Custom|ContractGrappleHook
  (bind _charactermovement (Variables|Character|GetCharacterMovement))
  ;[1 1 1] Contract Grapple Rope
  (Variables|GrappleHook|SetGrappleHooked false)
  (Variables|GrappleHook|SetIsGrappleHookContracting true)
  (Variables|/Script/Engine.CharacterMovementComponent|SetAirControl _charactermovement 0.0)
  (Variables|/Script/Engine.CharacterMovementComponent|SetGravityScale _charactermovement 0.0)
  (Character|LaunchCharacter (Math|Vector|MakeVector 0.0 0.0 (Variables|GrappleHook|GetGrappleInitialJumpSpeed)) false true)
  (Utilities|FlowControl|Delay (Variables|GrappleHook|GetGrappleInitialJumpTime))
  (Character|LaunchCharacter (* (Math|Vector|Normalize (- (Variables|GrappleHook|GetGrappleHookLocation) (Transformation|GetActorLocation))) (Variables|GrappleHook|GetGrappleSpeed)) true true)
  (CallFunction|ContractGrappleRopeAnimation))

(event Custom|Contract%20Grapple%20Rope%20Animation
  ;[1 1 1] Contract Grapple Rope Animation
  (bind _curve (Timeline|Timeline%20-%20Contract%20Grapple%20Rope%20Animation PlayFromStart)
    (:Update
      (Variables|/Script/CableComponent.CableComponent|SetCableLength (Variables|Default|GetGrappleRope) (* _curve (Variables|GrappleHook|GetGrappleRopeLength))))
    (:Finished
      (Variables|GrappleHook|SetIsGrappleHookContracting false)
      (Variables|/Script/Engine.CharacterMovementComponent|SetGravityScale (Variables|Character|GetCharacterMovement) 1.0)
      (Rendering|SetVisibility (Variables|Default|GetGrappleRope) false false)
      (CallFunction|ResetGrappleHook))))

(event Custom|ResetClimb
  ;[1 1 1] Reset Climb
  (Variables|Climb|SetIsClimbing false)
  (Variables|Climb|SetIsTouchingWall false)
  (Variables|Climb|SetIsClimbInterrupted false)
  (Variables|Climb|SetClimbTime 0.0))