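; Player character Blueprint with air jump, cooldown dash, timed wall climb, charged bow shot and grappling hook.
; The hook traces from the camera, animates a cable with timelines, then reels in through repeated launches.
; While hooked beyond rope length, outward input and velocity are projected out to fake a taut rope.
; Tick drives climbing on Climbable-tagged actors and the rope correction; state flags gate abilities, and landing resets jump and climb.
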(event Custom|ResetAirJump
  ;[1 1 1] Air Jump
  (Variables|AirJump|SetCanAirJump true))

(event EventOnLanded
  (params (Hit :type Hit%20Result%20Structure%20%28by%20ref%29))
  ;[1 1 1] Event On Landed
  (CallFunction|ResetAirJump)
  (CallFunction|ResetClimb))

(event EventBeginPlay
  ;[1 1 1] Initialization
  (Variables|/Script/Engine.CharacterMovementComponent|SetAirControl (Variables|Character|GetCharacterMovement) (Variables|General|GetDefaultAirControl)))

(event EventTick
  (params (DeltaSeconds :type Float%20%28single-precision%29))
  ;[1 1 1] Event Tick
  (Variables|General|SetDeltaTime DeltaSeconds)
  (Utilities|FlowControl|Sequence
    (:then_0
      (|Climb))
    (:then_1
      (GrappleHook|AdjustVelocitywhenHooked))))

(event Input|ActionEvents|InputActionJump
  (params (Key :type Key%20Structure))
  ;[1 1 1] Air Jump
  (:Pressed
    (Variables|General|SetIsJumpKeyPressed true)
    (if (Math|Boolean|ORBoolean (Variables|GrappleHook-Status|GetGrappleHooked) (Variables|GrappleHook-Status|GetReachHookEnd) (Variables|GrappleHook-Status|GetIsHookContracting))
      (CallFunction|BreakGrappleHook))
    (bind _newparam (CallFunction|GroundCheck))
    (if _newparam
      (Character|Jump)
      (elif (Variables|AirJump|GetCanAirJump)
        (Variables|AirJump|SetCanAirJump false)
        (Character|LaunchCharacter (Math|Vector|MakeVector 0.0 0.0 (Variables|AirJump|GetAirJumpSpeed)) false true))))
  (:Released
    (Variables|General|SetIsJumpKeyPressed false)))

(event Input|ActionEvents|InputActionDash
  (params (Key :type Key%20Structure))
  ;[1 1 1] Dash
  (:Pressed
    (if (Variables|Dash|GetCanDash)
      (bind _returnvalue (CallFunction|DashCheck))
      (if _returnvalue
        (Character|LaunchCharacter (* (Math|Vector|GetForwardVector (Variables|Default|GetCamera)) (Variables|Dash|GetDashDistance)) true true)
        (Variables|Dash|SetCanDash false)
        (Utilities|FlowControl|Delay 0.03) ; If there is no deday, character will keep moving and won't be stopped by the next node
        (Components|Movement|StopMovementImmediately (Variables|Character|GetCharacterMovement))
        (Utilities|FlowControl|Delay (Variables|Dash|GetDashCooldown))
        (Variables|Dash|SetCanDash true)))))

(event Input|ActionEvents|InputActionGrappleHook
  (params (Key :type Key%20Structure))
  ;[1 1 1] GrappleHook
  (:Pressed
    (|GrappleHook)))

(event Input|ActionEvents|InputActionFire
  (params (Key :type Key%20Structure))
  ;[1 1 1] Shoot Arrow
  (:Pressed
    (bind _returnvalue (CallFunction|ShootCheck))
    (if _returnvalue
      (|ShootArrow :!label _label)))
  (:Released
    (if (Variables|Arrow|GetHoldFire)
      (goto _label Released))))

(event Input|AxisEvents|InputAxisMouseLookHorizontal
  (params (AxisValue :type Float%20%28single-precision%29))
  ;[1 1 1] Character Orientation
  (Pawn|Input|AddControllerYawInput AxisValue))

(event Input|AxisEvents|InputAxisMouseLookVertical
  (params (AxisValue :type Float%20%28single-precision%29))
  ;[1 1 1] Character Orientation
  (Pawn|Input|AddControllerPitchInput AxisValue))

(event Input|AxisEvents|InputAxisHorizontalMovement
  (params (AxisValue :type Float%20%28single-precision%29))
  ;[1 1 1] Character Movement
  (if (|IsNotActuallyClimbing)
    (bind (_adjustedvector _adjustedvalue) (GrappleHook|GrappleHookMovementConstraint (Math|Vector|GetRightVector (Math|Rotator|MakeRotator 0.0 0.0 (.yaw (Pawn|GetControlRotation :!class /Script/Engine.Pawn)))) AxisValue))
    (Pawn|Input|AddMovementInput _adjustedvector _adjustedvalue false)))

(event Input|AxisEvents|InputAxisVerticalMovement
  (params (AxisValue :type Float%20%28single-precision%29))
  ;[1 1 1] Character Movement
  (bind (_adjustedvector _adjustedvalue) (GrappleHook|GrappleHookMovementConstraint (Math|Vector|GetForwardVector (Math|Rotator|MakeRotator 0.0 0.0 (.yaw (Pawn|GetControlRotation :!class /Script/Engine.Pawn)))) AxisValue))
  (Pawn|Input|AddMovementInput _adjustedvector _adjustedvalue false)
  (if (> AxisValue 0.0)
    (Variables|General|SetIsMovingForward true)
    (else
      (Variables|General|SetIsMovingForward false))))

(fn ConstructionScript)

(fn GroundCheck
  (bind (_outhit _returnvalue) (Collision|LineTraceByChannel (Transformation|GetActorLocation) (Transformation|GetWorldLocation (Variables|Default|GetGroundHitLocation)) "TraceTypeQuery1" false 0 "None"))
  (if _returnvalue
    (if (Utilities|Enum|Equal(Enum) (Collision|GetCollisionObjectType (.hitcomponent _outhit)) "ECC_WorldStatic")
      (LocalVariables|SetReturnValue true)))
  (return (LocalVariables|GetReturnValue)))

(fn CalculateGrappleHookDistance
  (bind _grapplerope (Variables|Default|GetGrappleRope))
  (bind _hooklocation (Variables|GrappleHook|GetHookLocation))
  (bind _returnvalue (Transformation|GetWorldLocation _grapplerope))
  (bind _returnvalue_2 (Math|Vector|Distance(Vector) _returnvalue _hooklocation))
  (Development|PrintString (Utilities|String|Append "Grapple Hook Distance: " (Utilities|String|ToString(Float) _returnvalue_2)) false)
  (return _returnvalue_2))

(fn GrappleHookMovementConstraint
  (params (Vector :type Vector) (Value :type Float%20%28single-precision%29))
  (LocalVariables|SetRawScale Value)
  (LocalVariables|SetRawVector Vector)
  (if (or (Variables|GrappleHook-Status|GetGrappleHooked) (Variables|GrappleHook-Status|GetReachHookEnd))
    (bind _returnvalue (GrappleHook|CalculateGrappleHookDistance))
    (Variables|GrappleHook|SetHookDistance _returnvalue)
    (if (> (Variables|GrappleHook|GetHookDistance) (Variables|GrappleHook|GetRopeLength))
      (LocalVariables|SetNormalizedGrappleHookVector (|CalculateNormalizedGrappleHookVector))
      (if (< (LocalVariables|GetRawScale) 0.0)
        (LocalVariables|SetRawVector (* (LocalVariables|GetRawVector) -1.0)))
      (bind _output_get (LocalVariables|SetIsOutwards (< (Math|Vector|DotProduct (LocalVariables|GetRawVector) (LocalVariables|GetNormalizedGrappleHookVector)) 0.0)))
      (if _output_get
        (if (== (LocalVariables|GetRawScale) 0.0)
          (return (- (LocalVariables|GetRawVector) (* (LocalVariables|GetNormalizedGrappleHookVector) (Math|Vector|DotProduct (LocalVariables|GetRawVector) (LocalVariables|GetNormalizedGrappleHookVector)))) 0.0)
          (else
            (return (- (LocalVariables|GetRawVector) (* (LocalVariables|GetNormalizedGrappleHookVector) (Math|Vector|DotProduct (LocalVariables|GetRawVector) (LocalVariables|GetNormalizedGrappleHookVector)))) 1.0)))
        (elif (< (LocalVariables|GetRawScale) 0.0)
          (return (* (LocalVariables|GetRawVector) -1.0) (LocalVariables|GetRawScale))
          (else
            (return (LocalVariables|GetRawVector) (LocalVariables|GetRawScale)))))
      (else
        (return (LocalVariables|GetRawVector) (LocalVariables|GetRawScale))))
    (else
      (return (LocalVariables|GetRawVector) (LocalVariables|GetRawScale)))))

(fn DashCheck
  (return (not (Math|Boolean|ORBoolean (Variables|Climb|GetIsTouchingWall) (Variables|GrappleHook-Status|GetIsHooking) (Variables|GrappleHook-Status|GetGrappleHooked) (Variables|GrappleHook-Status|GetIsHookContracting) (Variables|GrappleHook-Status|GetReachHookEnd)))))

(fn ShootCheck
  (return (not (Math|Boolean|ORBoolean (Variables|Climb|GetIsTouchingWall) (Variables|GrappleHook-Status|GetIsHooking) (Variables|GrappleHook-Status|GetIsHookContracting)))))

(fn AdjustVelocitywhenHooked
  (bind _returnvalue (Transformation|GetVelocity))
  (bind _returnvalue_2 (Transformation|GetActorLocation))
  (bind _hooklocation (Variables|GrappleHook|GetHookLocation))
  (bind _returnvalue_3 (- _returnvalue_2 _hooklocation))
  (bind _returnvalue_4 (Math|Vector|Normalize _returnvalue_3))
  (bind _returnvalue_5 (Math|Vector|DotProduct _returnvalue _returnvalue_4))
  ;[1 1 1] Condition Check
  (if (or (Variables|GrappleHook-Status|GetGrappleHooked) (Variables|GrappleHook-Status|GetReachHookEnd))
    (bind _returnvalue_6 (GrappleHook|CalculateGrappleHookDistance))
    (Variables|GrappleHook|SetHookDistance _returnvalue_6)
    (if (> (Variables|GrappleHook|GetHookDistance) (Variables|GrappleHook|GetRopeLength))
      ;[1 1 1] Adjust Velocity to Get Rid of Centrifugal Velocity
      (if (not (< _returnvalue_5 0.0))
        (Variables|/Script/Engine.MovementComponent|SetVelocity (Variables|Character|GetCharacterMovement) (- _returnvalue (* _returnvalue_4 _returnvalue_5)))))))

(event OnComponentHit(CapsuleComponent)
  (params (HitComponent :type Primitive%20Component%20Object%20Reference) (OtherActor :type Actor%20Object%20Reference) (OtherComp :type Primitive%20Component%20Object%20Reference) (NormalImpulse :type Vector :default "0, 0, 0") (Hit :type Hit%20Result%20Structure%20%28by%20ref%29))
  ;[1 1 1] Deprecated: Extra Jump At the End of Grapple
)

(event Custom|ResetGrappleHook
  (bind _grapplerope (Variables|Default|GetGrappleRope))
  ;[1 1 1] Reset Grapple Hook
  (Variables|/Script/Engine.CharacterMovementComponent|SetAirControl (Variables|Character|GetCharacterMovement) (Variables|General|GetDefaultAirControl))
  (Class|CableComponent|SetAttachEndto _grapplerope 0 "None" "None")
  (Variables|/Script/CableComponent.CableComponent|SetEndLocation _grapplerope "0, 0, 0")
  (Variables|/Script/CableComponent.CableComponent|SetbAttachEnd _grapplerope true)
  (bind _output_get (Variables|GrappleHook|SetRopeLength 0.0))
  (Variables|/Script/CableComponent.CableComponent|SetCableLength _grapplerope _output_get) ; Cable length has already been set to zero in the break grapple hook timeline
  (Utilities|FlowControl|Delay (Variables|GrappleHook|GetHookCooldown))
  (Variables|GrappleHook|SetCanGrappleHook true))

(event Custom|ShootGrappleHookAnimation
  (bind _grapplerope (Variables|Default|GetGrappleRope))
  (bind _grapplerope_2 (Variables|Default|GetGrappleRope))
  ;[1 1 1] Shoot Grapple Hook Animation
  (Rendering|SetVisibility _grapplerope true false)
  (if (Variables|GrappleHook|GetGrappleHookHit)
    (Class|CableComponent|SetAttachEndto _grapplerope (Variables|GrappleHook|GetHookActor) "None" "None")
    (bind _curve (Timeline|Timeline%20-%20Shoot%20Grapple%20Hook PlayFromStart) ; It takes 0.3s for grapple hook to reach its end
      (:Update
        (|UpdateRopeEndLocation _curve))
      (:Finished
        (Variables|/Script/CableComponent.CableComponent|SetCableLength _grapplerope_2 (Variables|GrappleHook|GetRopeLength))
        (Variables|GrappleHook-Status|SetIsHooking false)
        (if (Variables|GrappleHook|GetGrappleHookHit)
          (Variables|GrappleHook-Status|SetGrappleHooked true)
          (Variables|/Script/Engine.CharacterMovementComponent|SetAirControl (Variables|Character|GetCharacterMovement) 1.0)
          (else
            (Variables|/Script/CableComponent.CableComponent|SetbAttachEnd _grapplerope_2 false)
            (CallFunction|BreakGrappleHookAnimation)))))
    (else
      (Timeline|Timeline%20-%20Shoot%20Grapple%20Hook PlayFromStart))))

(event Custom|ShootGrappleHook
  (bind _camera (Variables|Default|GetCamera))
  (bind _returnvalue (Transformation|GetWorldLocation _camera))
  ;[1 1 1] Check for Surface
  (if (Variables|GrappleHook|GetCanGrappleHook)
    (Variables|GrappleHook|SetCanGrappleHook false)
    (Variables|GrappleHook-Status|SetIsHooking true)
    (bind _output_get (Variables|GrappleHook|SetHookLocation (+ _returnvalue (* (Math|Vector|GetForwardVector _camera) (Variables|GrappleHook|GetHookRange)))))
    (bind (_outhit _returnvalue_2) (Collision|LineTraceByChannel _returnvalue _output_get "TraceTypeQuery3" false 0 "ForDuration"))
    ;[1 1 1] Store Rope Information
    (bind _output_get_2 (Variables|GrappleHook|SetGrappleHookHit _returnvalue_2))
    (Variables|GrappleHook|SetHookActor (.hitactor _outhit))
    (if _output_get_2
      (Variables|GrappleHook|SetHookLocation (.location _outhit))
      (Variables|GrappleHook|SetRopeLength (+ (.distance _outhit) (Variables|GrappleHook|GetLengthPadding)))
      (else
        (Variables|GrappleHook|SetRopeLength (Variables|GrappleHook|GetHookRange))))
    (CallFunction|ShootGrappleHookAnimation)))

(event Custom|ReachGrappleHookEnd
  (bind _charactermovement (Variables|Character|GetCharacterMovement))
  ;[1 1 1] Reach Grapple Hook End
  (Utilities|Time|ClearandInvalidateTimerbyHandle (Variables|GrappleHook|GetEndContractionTimer))
  (Components|Movement|StopMovementImmediately _charactermovement)
  (Variables|/Script/Engine.CharacterMovementComponent|SetAirControl _charactermovement 1.0) ; Set air control to 1 again just in case
  (bind _returnvalue (GrappleHook|CalculateGrappleHookDistance))
  (bind _output_get (Variables|GrappleHook|SetRopeLength _returnvalue))
  (Variables|/Script/CableComponent.CableComponent|SetCableLength (Variables|Default|GetGrappleRope) _output_get)
  (Variables|GrappleHook-Status|SetReachHookEnd true)
  (Variables|GrappleHook-Status|SetIsHookContracting false))

(event Custom|ContractGrappleHook
  ;[1 1 1] Contract Grapple Hook
  (Variables|GrappleHook-Status|SetGrappleHooked false)
  (Variables|GrappleHook-Status|SetIsHookContracting true)
  (Variables|/Script/Engine.CharacterMovementComponent|SetAirControl (Variables|Character|GetCharacterMovement) 1.0)
  (Character|LaunchCharacter (Math|Vector|MakeVector 0.0 0.0 (Variables|GrappleHook|GetInitialJumpSpeed)) false true)
  (Utilities|FlowControl|Delay (Variables|GrappleHook|GetInitialJumpTime))
  (bind _returnvalue (Utilities|Time|SetTimerbyEvent (delegate Custom|ReachGrappleHookEnd) (Variables|GrappleHook|GetMaxContractionTime)))
  (Variables|GrappleHook|SetEndContractionTimer _returnvalue)
  (if (Variables|GrappleHook-Status|GetIsHookContracting) :!label _label
    (bind _returnvalue_2 (GrappleHook|CalculateGrappleHookDistance))
    (if (<= _returnvalue_2 (Variables|GrappleHook|GetHookCloseRange))
      (CallFunction|ReachGrappleHookEnd)
      (else
        (bind _output_get (Variables|GrappleHook|SetHookDistance _returnvalue_2))
        (Variables|/Script/CableComponent.CableComponent|SetCableLength (Variables|Default|GetGrappleRope) _output_get)
        (Character|LaunchCharacter (* (Math|Vector|Normalize (- (Variables|GrappleHook|GetHookLocation) (Transformation|GetActorLocation))) (Variables|GrappleHook|GetHookContractSpeed)) true true)
        (Utilities|FlowControl|Delay (Variables|General|GetDeltaTime))
        (goto _label)))))

(event Custom|BreakGrappleHook
  ;[1 1 1] Break Grapple Hook
  (Variables|GrappleHook-Status|SetGrappleHooked false)
  (Variables|GrappleHook-Status|SetIsHookContracting false)
  (Variables|GrappleHook-Status|SetReachHookEnd false)
  (Variables|/Script/CableComponent.CableComponent|SetbAttachEnd (Variables|Default|GetGrappleRope) false)
  (CallFunction|BreakGrappleHookAnimation))

(event Custom|Break%20Grapple%20Hook%20Animation
  ;[1 1 1] Break Grapple Hook Animation
  (bind _curve (Timeline|Timeline%20-%20Break%20Grapple%20Hook PlayFromStart)
    (:Update
      (Variables|/Script/CableComponent.CableComponent|SetCableLength (Variables|Default|GetGrappleRope) (* _curve (Variables|GrappleHook|GetRopeLength))))
    (:Finished
      (Rendering|SetVisibility (Variables|Default|GetGrappleRope) false false)
      (CallFunction|ResetGrappleHook))))

(event Custom|ResetClimb
  ;[1 1 1] Reset Climb
  (Variables|Climb|SetClimbStarted false)
  (Variables|Climb|SetIsTouchingWall false)
  (Variables|Climb|SetClimbInterrupted false)
  (Variables|Climb|SetClimbTime 0.0))